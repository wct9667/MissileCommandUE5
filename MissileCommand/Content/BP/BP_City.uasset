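; BP_City is a city target that a missile can destroy, built from four cube components, a box trigger and an explosion effect.
; The first BP_Missile to overlap the box sets a Destroyed flag, hides the cubes and activates NSExplosionCity.
; The flag blocks later hits, and the actor itself is not removed from the level.
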(event `self.Box.OnComponentBeginOverlap`
  (params (OverlappedComponent :type "PrimitiveComponent Object Reference") (OtherActor :type "Actor Object Reference") (OtherComp :type "PrimitiveComponent Object Reference") (OtherBodyIndex :type Integer) (bFromSweep :type Boolean) (SweepResult :type "HitResult Structure (by ref)"))
  (if (not (`self.Destroyed`))
    (cast `/Game/BP/BP_Missile` OtherActor)
    (set `self.Destroyed` true)
    (`SceneComponent.SetVisibility` (`self.Cube`) false false)
    (`SceneComponent.SetVisibility` (`self.Cube3`) false false)
    (`SceneComponent.SetVisibility` (`self.Cube4`) false false)
    (`SceneComponent.SetVisibility` (`self.Cube2`) false false)
    (`ActorComponent.Activate` (`self.NS_ExplosionCity`) false)))

(fn `UserConstructionScript`)