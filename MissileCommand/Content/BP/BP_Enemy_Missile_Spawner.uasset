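; Enemy missile spawner that periodically launches waves of BP_Missile actors at random targets.
; Tick accumulates time and, each time SpawnRate elapses, runs a spawn loop sized by a random pick from NumberToSpawn.
; Each missile spawns at a random point inside the Box component's bounds.
; SpawnMissile gives it the current location of a random Targets entry as a fixed aim point, plus a reference back to the spawner.
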(event `self.ReceiveTick`
  (params (DeltaSeconds :type "Float (single-precision)"))
  (bind (_origin _boxextent) (`KismetSystemLibrary.GetComponentBounds` (`self.Box`)))
  ; Spawn Every SpawnRate seconds
  (bind _output_get (set `self.TimeBetweenSpawns` (+ DeltaSeconds (`self.TimeBetweenSpawns`))))
  (if (>= _output_get (`self.SpawnRate`))
    (set `self.TimeBetweenSpawns` 0.0)
    (for _ (range (+ (`KismetMathLibrary.FTrunc` (`KismetArrayLibrary.Array_Random` (`self.NumberToSpawn`))) 1))
      (`self.SpawnMissile` (`KismetMathLibrary.Conv_VectorToTransform` (`KismetMathLibrary.RandomPointInBoundingBox` _origin _boxextent))))))

(fn `SpawnMissile`
  (params (SpawnTransform :type "Transform Structure"))
  (bind _returnvalue (`|SpawnActorFromClass` "/Game/BP/BP_Missile.BP_Missile_C" SpawnTransform "Undefined" "MultiplyWithRoot" null null))
  (set `/Game/BP/BP_Missile.Target` (`self.K2_GetActorLocation` (`KismetArrayLibrary.Array_Random` (`self.Targets`))) _returnvalue)
  (set `/Game/BP/BP_Missile.SpawnerRef` self _returnvalue))

(fn `UserConstructionScript`)