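; BP_Missile is an actor that flies toward a target point and can split into two new missiles mid-flight.
; Tick rotates and moves it at constant speed, and at or above zero height periodically rolls against a split chance randomized at BeginPlay.
; A split spawns both replacements through SpawnerRef.
; Overlaps with non-missiles trigger an explosion; both endings fade the particle trail before delayed destruction.
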(event `Destroy`
  ; DEstroys a missile, spawning in proper particle effects and then deletes itself
  (`NiagaraComponent.SetVariableFloat` (`self.Missile`) "Emmision" 0.0)
  (`NiagaraComponent.SetVariableVec3` (`self.Missile`) "Velocity Scale" (0.1 0.1 0.1))
  (`ActorComponent.Activate` (`self.Explosion`) false)
  (set `self.Destroyed` true)
  (`KismetSystemLibrary.Delay` 6.0)
  (`self.K2_DestroyActor`))

(event `self.ReceiveBeginPlay`
  ; Get a random chance to split
  (bind _output_get (set `self.SplitChance` (`KismetMathLibrary.RandomFloatInRange` 0.0 (`self.MaxSplitChance`))))
  (`KismetSystemLibrary.PrintString` (`KismetStringLibrary.Conv_DoubleToString` _output_get)))

(event `self.Collider.OnComponentBeginOverlap`
  (params (OverlappedComponent :type "PrimitiveComponent Object Reference") (OtherActor :type "Actor Object Reference") (OtherComp :type "PrimitiveComponent Object Reference") (OtherBodyIndex :type Integer) (bFromSweep :type Boolean) (SweepResult :type "HitResult Structure (by ref)"))
  (cast `/Game/BP/BP_Missile` OtherActor
    (:`CastFailed`
      (`self.Destroy`))))

(event `self.ReceiveTick`
  (params (DeltaSeconds :type "Float (single-precision)"))
  (if (not (`self.Destroyed`))
    (`self.MoveTowardsTarget` DeltaSeconds)
    (`self.ChanceToSplit` DeltaSeconds)))

(event `ChanceToSplit`
  (params (DeltaTime :type "Float (double-precision)"))
  (bind (_returnvalue_x _returnvalue_y _returnvalue_z) (`KismetMathLibrary.BreakVector` (`self.K2_GetActorLocation`)))
  ; This long ass function randomly has achance to split the missile, when it does it destroys the old on after a delay and removes it emmision.
  (if (>= _returnvalue_z 0.0)
    (set `self.SplitTimer` (+ DeltaTime (`self.SplitTimer`)))
    (if (>= (`self.SplitTimer`) (`self.SplitRate`))
      (set `self.SplitTimer` 0.0)
      (if true
        (if (<= (`KismetMathLibrary.RandomFloatInRange` 0.0 100.0) (`self.SplitChance`))
          (`self.SpawnMissileOnSelf`)
          (`self.SpawnMissileOnSelf`)
          (`NiagaraComponent.SetVariableFloat` (`self.Missile`) "Emmision" 0.0)
          (`NiagaraComponent.SetVariableVec3` (`self.Missile`) "Velocity Scale" (0.1 0.1 0.1))
          (set `self.Destroyed` true)
          (`KismetSystemLibrary.Delay` 6.0)
          (`self.K2_DestroyActor`))))))

(fn `MoveTowardsTarget`
  (params (DeltaTime :type "Float (double-precision)"))
  (`self.K2_SetActorRotation` self (`KismetMathLibrary.FindLookAtRotation` (`self.K2_GetActorLocation`) (`self.Target`)) false)
  (`self.K2_SetActorLocation` (`KismetMathLibrary.VInterpTo_Constant` (`self.K2_GetActorLocation`) (`self.Target`) DeltaTime (`self.Speed`))))

(fn `SpawnMissileOnSelf`
  (`/Game/BP/BP_Enemy_Missile_Spawner.SpawnMissile` (`self.SpawnerRef`) (`self.GetTransform`)))

(fn `UserConstructionScript`)