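; Player-fired missile actor that flies toward a Target point until it is marked Destroyed.
; Tick rotates it to face Target and moves it at constant Speed; a signed Y/Z proximity check only prints debug text.
; Destroy stops the missile effect's emission, lowers its velocity scale, activates the explosion, then deletes the actor after a delay.
; Overlap handling is empty, and the silo-cast branch that calls Destroy is disconnected.
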(event `self.Collider.OnComponentBeginOverlap`
  (params (OverlappedComponent :type "PrimitiveComponent Object Reference") (OtherActor :type "Actor Object Reference") (OtherComp :type "PrimitiveComponent Object Reference") (OtherBodyIndex :type Integer) (bFromSweep :type Boolean) (SweepResult :type "HitResult Structure (by ref)")))

(event `self.ReceiveBeginPlay`)

(event `self.ReceiveTick`
  (params (DeltaSeconds :type "Float (single-precision)"))
  (bind _returnvalue_location (`KismetMathLibrary.BreakTransform` (`self.GetTransform`)))
  (bind (_returnvalue_x _returnvalue_y _returnvalue_z) (`KismetMathLibrary.BreakVector` (- (`self.Target`) _returnvalue_location)))
  (if (not (`self.Destroyed`))
    (`self.MoveTowardsTarget` DeltaSeconds)
    (if (<= _returnvalue_y 5.0)
      (if (<= _returnvalue_z 5.0)
        (`KismetSystemLibrary.PrintString` "At target!")))))

(event `Destroy`
  ; DEstroys a missile, spawning in proper particle effects and then deletes itself
  (`NiagaraComponent.SetVariableFloat` (`self.Missile`) "Emmision" 0.0)
  (`NiagaraComponent.SetVariableVec3` (`self.Missile`) "Velocity Scale" (0.1 0.1 0.1))
  (`ActorComponent.Activate` (`self.Explosion`) false)
  (set `self.Destroyed` true)
  (`KismetSystemLibrary.Delay` 6.0)
  (`self.K2_DestroyActor`))

(fn `MoveTowardsTarget`
  (params (DeltaTime :type "Float (double-precision)"))
  (`self.K2_SetActorRotation` self (`KismetMathLibrary.FindLookAtRotation` (`self.K2_GetActorLocation`) (`self.Target`)) false)
  (`self.K2_SetActorLocation` (`KismetMathLibrary.VInterpTo_Constant` (`self.K2_GetActorLocation`) (`self.Target`) DeltaTime (`self.Speed`)))
  (`KismetSystemLibrary.PrintString` (`KismetStringLibrary.Conv_VectorToString` (`self.Target`))))

(fn `UserConstructionScript`)