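; Countdown timer actor that shows time on a TextRender and brings up the win UI at zero.
; BeginPlay starts a 15-second countdown through a looping one-second timer, with reusable functions to set, start, pause and clear it in either direction.
; Each step updates the text and, on hitting the goal, clears the timer and fires OnTimerReachedGoal.
; Tick separately adds a new BP_UI_Win every frame while time is at or below the goal.
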(event `self.ReceiveBeginPlay`
  (`self.SetGoal` 0)
  (`self.SetTime` 0 0 15)
  (`self.StartTimer` false))

(event `self.ReceiveTick`
  (params (DeltaSeconds :type "Float (single-precision)"))
  (if (<= (`self.Time`) (`self.TimeGoal`))
    (bind _returnvalue (`|CreateWidget` "/Game/BP/UI/BP_UI_Win.BP_UI_Win_C"))
    (`UserWidget.AddToViewport` _returnvalue 0)))

(fn `ClearTimer`
  (`KismetSystemLibrary.K2_ClearAndInvalidateTimerHandle` (`self.TimerHandle`)))

(fn `PauseTimer`
  (bind _timerhandle (`self.TimerHandle`))
  (if (`KismetSystemLibrary.K2_IsValidTimerHandle` _timerhandle)
    (`KismetSystemLibrary.K2_PauseTimerHandle` _timerhandle)))

(fn `SetGoal`
  (params (Hours :type Integer) (Minutes :type Integer) (Seconds :type Integer) (GoalText :type "Text (by ref)"))
  (set `self.TimeGoal` (`KismetMathLibrary.MakeTimespan` 0 Hours Minutes Seconds))
  (`TextRenderComponent.K2_SetText` (`self.TextRender`) GoalText))

(fn `SetTime`
  (params (Hours :type Integer) (Minutes :type Integer) (Seconds :type Integer))
  (bind _output_get (set `self.Time` (`KismetMathLibrary.MakeTimespan` 0 Hours Minutes Seconds)))
  (bind (_days _hours _minutes _seconds) (`KismetMathLibrary.BreakTimespan` _output_get))
  (if (== _hours 0)
    (`TextRenderComponent.K2_SetText` (`self.TextRender`) (`|FormatText` "{Minute}:{Second}" (`KismetTextLibrary.Conv_IntToText` _minutes false true 2) (`KismetTextLibrary.Conv_IntToText` _seconds false true 2)))
    (else
      (bind (_days_2 _hours_2 _minutes_2 _seconds_2) (`KismetMathLibrary.BreakTimespan` _output_get))
      (`TextRenderComponent.K2_SetText` (`self.TextRender`) (`|FormatText` "{Hour}:{Minute}:{Second}" (`KismetTextLibrary.Conv_IntToText` _hours_2 false true 2) (`KismetTextLibrary.Conv_IntToText` _minutes_2 false true 2) (`KismetTextLibrary.Conv_IntToText` _seconds_2 false true 2))))))

(fn `StartTimer`
  (params (bForward :type Boolean))
  (set `self.bForward` bForward)
  (if (`KismetSystemLibrary.K2_IsValidTimerHandle` (`self.TimerHandle`))
    (`KismetSystemLibrary.K2_UnPauseTimerHandle` (`self.TimerHandle`))
    (else
      (bind _returnvalue (`KismetSystemLibrary.K2_SetTimer` null "UpdateEachSecond" 1.0 true))
      (set `self.TimerHandle` _returnvalue))))

(fn `UpdateEachSecond`
  (bind (_days _hours _minutes _seconds) (`KismetMathLibrary.BreakTimespan` (+ (`self.Time`) (`KismetMathLibrary.MakeTimespan` 0 0 0 (select `bool` (`self.bForward`) :`false` -1 :`true` 1)))))
  (`self.SetTime` _hours _minutes _seconds)
  (if (== (`self.Time`) (`self.TimeGoal`))
    (`|ExecutionSequence`
      (:`then_0`
        (`self.ClearTimer`))
      (:`then_1`
        (`self.OnTimerReachedGoal`)))))

(fn `UserConstructionScript`)