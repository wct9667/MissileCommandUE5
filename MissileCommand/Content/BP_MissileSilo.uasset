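; BP_MissileSilo is a destructible missile silo that holds ammo and supplies a launch point for missiles.
; A BP_Missile overlapping its Box marks it Destroyed once, hides the silo mesh and ammo text, and activates a Niagara effect.
; SubtractAmmo decrements a clamped count, refreshes the text display and flags OutOfAmmo at zero, while GetLaunchLocation returns the MissileMouth world position.
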(event `self.Box.OnComponentBeginOverlap`
  (params (OverlappedComponent :type "PrimitiveComponent Object Reference") (OtherActor :type "Actor Object Reference") (OtherComp :type "PrimitiveComponent Object Reference") (OtherBodyIndex :type Integer) (bFromSweep :type Boolean) (SweepResult :type "HitResult Structure (by ref)"))
  (if (not (`self.Destroyed`))
    (cast `/Game/BP/BP_Missile` OtherActor)
    (set `self.Destroyed` true)
    (`SceneComponent.SetVisibility` (`self.Silo`) false false)
    (`ActorComponent.Activate` (`self.Niagara`) false)
    (`SceneComponent.SetVisibility` (`self.MissileText`) false false)))

(event `self.ReceiveBeginPlay`
  (`TextRenderComponent.K2_SetText` (`self.MissileText`) (`KismetTextLibrary.Conv_IntToText` (`self.Ammo`))))

(fn `GetLaunchLocation`
  (returns (LaunchLocation :type "Vector Structure"))
  (return (`SceneComponent.K2_GetComponentLocation` (`self.Missile Mouth`))))

(fn `SubtractAmmo`
  (set `self.Ammo` (`KismetMathLibrary.Clamp` (- (`self.Ammo`) 1) 0 1000))
  (`self.UpdateAmmoText`)
  (if (<= (`self.Ammo`) 0)
    (set `self.OutOfAmmo` true)))

(fn `UpdateAmmoText`
  (`TextRenderComponent.K2_SetText` (`self.MissileText`) (`KismetTextLibrary.Conv_IntToText` (`self.Ammo`))))

(fn `UserConstructionScript`)