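; Player pawn that prototypes Enhanced Input controls for aiming and firing two silos.
; On controller change it adds the IMC mapping context to the player's input subsystem and prints the most recently used device type.
; The aim action moves the whole actor by the negated, axis-swapped input, with no sweep or delta-time scaling.
; Both fire actions and a test action only print debug strings.
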(event `self.ReceiveControllerChanged`
  (params (OldController :type "Controller Object Reference") (NewController :type "Controller Object Reference"))
  (bind _asplayer_controller (cast `PlayerController` NewController))
  (`EnhancedInputSubsystemInterface.AddMappingContext` (pcsubsystem `EnhancedInputLocalPlayerSubsystem` _asplayer_controller) "/Game/PlayerInput/IMC.IMC" 0 (struct))
  (`KismetSystemLibrary.PrintString` "Hello")
  (`KismetSystemLibrary.PrintString` (`|GetEnumeratorNameAsString` (`.PrimaryDeviceType` (break `HardwareDeviceIdentifier` (`InputDeviceSubsystem.GetMostRecentlyUsedHardwareDevice` :`self` (subsystem `InputDeviceSubsystem`)))))))

(event `EnhancedInput|/Game/PlayerInput/IA_FireSilo1`
  (params (ActionValue :type "Float (double-precision)") (ElapsedSeconds :type "Float (double-precision)") (TriggeredSeconds :type "Float (double-precision)") (InputAction :type "InputAction Object Reference" :default "/Game/PlayerInput/IA_FireSilo1.IA_FireSilo1"))
  ;[0.05098 0.05098 0.05098] Fire Input
  (:`Triggered`
    (`KismetSystemLibrary.PrintString` "Fire Silo 1")))

(event `EnhancedInput|/Game/PlayerInput/IA_FireSilo2`
  (params (ActionValue :type "Float (double-precision)") (ElapsedSeconds :type "Float (double-precision)") (TriggeredSeconds :type "Float (double-precision)") (InputAction :type "InputAction Object Reference" :default "/Game/PlayerInput/IA_FireSilo2.IA_FireSilo2"))
  ;[0.05098 0.05098 0.05098] Fire Input
  (:`Triggered`
    (`KismetSystemLibrary.PrintString` "Fire Silo 2")))

(event `EnhancedInput|/Game/PlayerInput/IA_AIM`
  (params (ActionValue :type "Vector Structure") (ElapsedSeconds :type "Float (double-precision)") (TriggeredSeconds :type "Float (double-precision)") (InputAction :type "InputAction Object Reference" :default "/Game/PlayerInput/IA_AIM.IA_AIM"))
  (bind (_returnvalue_x _returnvalue_y _returnvalue_z) (`KismetMathLibrary.BreakVector` (* ActionValue (-1.0 -1.0 -1.0))))
  ;[0.05098 0.05098 0.05098] Aim Input
  (:`Triggered`
    (`self.K2_SetActorLocation` (+ (`KismetMathLibrary.MakeVector` _returnvalue_z _returnvalue_x _returnvalue_y) (`self.K2_GetActorLocation`)))
    (`KismetSystemLibrary.PrintString` "Aim")))

(event `EnhancedInput|/Game/PlayerInput/IA_Test`
  (params (ActionValue :type "Float (double-precision)") (ElapsedSeconds :type "Float (double-precision)") (TriggeredSeconds :type "Float (double-precision)") (InputAction :type "InputAction Object Reference" :default "/Game/PlayerInput/IA_Test.IA_Test"))
  (:`Triggered`
    (`KismetSystemLibrary.PrintString` "Hello")))

(fn `UserConstructionScript`)